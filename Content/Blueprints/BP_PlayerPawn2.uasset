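; BP_PlayerPawn2 is a player pawn that turns Enhanced Input actions into skill casts.
; The shoot, summon wall and cone blast actions each call the matching function on its BPSkillSystem, passing the SpiritBallLocation component's world location and rotation.
; An unconnected node chain for adding a mapping context to the owning player controller's input subsystem never runs.
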(event `EnhancedInput|/Game/Input/IA_Shoot`
  (params (ActionValue :type Boolean) (ElapsedSeconds :type "Float (double-precision)") (TriggeredSeconds :type "Float (double-precision)") (InputAction :type "InputAction Object Reference" :default "/Game/Input/IA_Shoot.IA_Shoot"))
  (bind _spiritballlocation (`self.SpiritBallLocation`))
  (:`Triggered`
    (`/Game/Blueprints/BP_SkillSystem.Shoot` (`self.BP_SkillSystem`) (`SceneComponent.K2_GetComponentLocation` _spiritballlocation) (`SceneComponent.K2_GetComponentRotation` _spiritballlocation))))

(event `EnhancedInput|/Game/Input/IA_SummonWall`
  (params (ActionValue :type Boolean) (ElapsedSeconds :type "Float (double-precision)") (TriggeredSeconds :type "Float (double-precision)") (InputAction :type "InputAction Object Reference" :default "/Game/Input/IA_SummonWall.IA_SummonWall"))
  (bind _spiritballlocation (`self.SpiritBallLocation`))
  (:`Triggered`
    (`/Game/Blueprints/BP_SkillSystem.SummonWall` (`self.BP_SkillSystem`) (`SceneComponent.K2_GetComponentLocation` _spiritballlocation) (`SceneComponent.K2_GetComponentRotation` _spiritballlocation))))

(event `EnhancedInput|/Game/Input/IA_ConeBlast`
  (params (ActionValue :type Boolean) (ElapsedSeconds :type "Float (double-precision)") (TriggeredSeconds :type "Float (double-precision)") (InputAction :type "InputAction Object Reference" :default "/Game/Input/IA_ConeBlast.IA_ConeBlast"))
  (bind _spiritballlocation (`self.SpiritBallLocation`))
  (:`Triggered`
    (`/Game/Blueprints/BP_SkillSystem.ConeBlast` (`self.BP_SkillSystem`) (`SceneComponent.K2_GetComponentLocation` _spiritballlocation) (`SceneComponent.K2_GetComponentRotation` _spiritballlocation))))

(fn `UserConstructionScript`)