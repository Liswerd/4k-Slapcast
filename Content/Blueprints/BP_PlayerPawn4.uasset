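; Player pawn that grants itself spirit ball, wall and cone spells on BeginPlay and handles their casting input.
; Wall and cone inputs play a grunt and call BPSkillSystem at the SpiritBallLocation transform.
; The pause input toggles a pause menu widget and the game's paused state.
; The shoot input is empty, with its casting logic and the input mapping context setup left disconnected.
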(event `self.ReceiveBeginPlay`
  (bind _returnvalue (`AddComponent|NODE_AddSpiritBall-2`))
  (`self.ExecAddMagicSpell` _returnvalue)
  (bind _returnvalue_2 (`AddComponent|NODE_AddWall-1`))
  (`self.ExecAddMagicSpell` _returnvalue_2)
  (bind _returnvalue_3 (`AddComponent|NODE_AddCone-1`))
  (`self.ExecAddMagicSpell` _returnvalue_3))

(event `EnhancedInput|/Game/Input/IA_Shoot`
  (params (ActionValue :type Boolean) (ElapsedSeconds :type "Float (double-precision)") (TriggeredSeconds :type "Float (double-precision)") (InputAction :type "InputAction Object Reference" :default "/Game/Input/IA_Shoot.IA_Shoot")))

(event `EnhancedInput|/Game/Input/IA_SummonWall`
  (params (ActionValue :type Boolean) (ElapsedSeconds :type "Float (double-precision)") (TriggeredSeconds :type "Float (double-precision)") (InputAction :type "InputAction Object Reference" :default "/Game/Input/IA_SummonWall.IA_SummonWall"))
  (bind _spiritballlocation (`self.SpiritBallLocation`))
  (bind _returnvalue (`SceneComponent.K2_GetComponentLocation` _spiritballlocation))
  (:`Triggered`
    (`GameplayStatics.PlaySoundAtLocation` "/Game/AudioFiles/PlayerGrunt_Cue.PlayerGrunt_Cue" _returnvalue (struct) 1.0 1.0 0.0 null null null null)
    (`/Game/Blueprints/BP_SkillSystem.SummonWall` (`self.BP_SkillSystem`) _returnvalue (`SceneComponent.K2_GetComponentRotation` _spiritballlocation))))

(event `EnhancedInput|/Game/Input/IA_ConeBlast`
  (params (ActionValue :type Boolean) (ElapsedSeconds :type "Float (double-precision)") (TriggeredSeconds :type "Float (double-precision)") (InputAction :type "InputAction Object Reference" :default "/Game/Input/IA_ConeBlast.IA_ConeBlast"))
  (bind _spiritballlocation (`self.SpiritBallLocation`))
  (bind _returnvalue (`SceneComponent.K2_GetComponentLocation` _spiritballlocation))
  (:`Triggered`
    (`GameplayStatics.PlaySoundAtLocation` "/Game/AudioFiles/PlayerGrunt_Cue.PlayerGrunt_Cue" _returnvalue (struct) 1.0 1.0 0.0 null null null null)
    (`/Game/Blueprints/BP_SkillSystem.ConeBlast` (`self.BP_SkillSystem`) _returnvalue (`SceneComponent.K2_GetComponentRotation` _spiritballlocation))))

(event `EnhancedInput|/Game/Input/IA_Pause`
  (params (ActionValue :type Boolean) (ElapsedSeconds :type "Float (double-precision)") (TriggeredSeconds :type "Float (double-precision)") (InputAction :type "InputAction Object Reference" :default "/Game/Input/IA_Pause.IA_Pause"))
  (:`Started`
    (if (not (`self.IsPauseMenuOpen`))
      (set `self.IsPauseMenuOpen` true)
      (bind _returnvalue (`|CreateWidget` "/Game/UI/PauseMenu.PauseMenu_C" (`GameplayStatics.GetPlayerController` 0)))
      (bind _output_get (set `self.PauseMenuWidget` _returnvalue))
      (`UserWidget.AddToViewport` _output_get 0)
      (`GameplayStatics.SetGamePaused` true)
      (else
        (set `self.IsPauseMenuOpen` false)
        (`Widget.RemoveFromParent` (`self.PauseMenuWidget`))
        (`GameplayStatics.SetGamePaused` false)))))

(fn `UserConstructionScript`)