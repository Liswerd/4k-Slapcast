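; Ranged enemy AI character that chases the player and attacks with spirit balls.
; Tick paths toward the player beyond 1000 units, otherwise stops and plays a DoOnce-gated attack montage, while facing the player and updating a camera-facing health bar.
; SpawnBall launches a projectile at the player; its caller is outside this graph.
; Overlapping player-owned castables deals damage until death, and random-interval grunts loop from BeginPlay.
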(event `SpawnBall`
  (bind _spiritballlocation (`self.SpiritBallLocation`))
  (bind _returnvalue (`|SpawnActorFromClass` "/Game/Blueprints/BP_SpiritBallObject.BP_SpiritBallObject_C" (`KismetMathLibrary.MakeTransform` (`SceneComponent.K2_GetComponentLocation` _spiritballlocation) (`SceneComponent.K2_GetComponentRotation` _spiritballlocation)) "AdjustIfPossibleButAlwaysSpawn" "MultiplyWithRoot" null null))
  (`/Game/Blueprints/BP_SpiritBallObject.SetVelocity` _returnvalue (* (`KismetMathLibrary.Normal` (- (`SceneComponent.K2_GetComponentLocation` (`Actor.RootComponent` (`GameplayStatics.GetPlayerPawn` 0))) (`SceneComponent.K2_GetComponentLocation` (`self.CapsuleComponent`)))) (`self.Speed`))))

(event `AttackPLayerForAnim`
  (`/Engine/EditorBlueprintResources/StandardMacros.DoOnce` false :!label _label
    (:`Completed`
      (bind _returnvalue (`self.PlayAnimMontage` "/Game/animations/shrivler_animations/ShrivlerFasterAttackMontage.ShrivlerFasterAttackMontage"))
      (`KismetSystemLibrary.Delay` _returnvalue)
      (set `self.CanAttack` true)
      (goto _label :!via `Reset`))))

(event `self.ReceiveBeginPlay`
  ; makes the sound effect for random grunts
  (`GameplayStatics.PlaySoundAtLocation` "/Game/AudioFiles/ZombieGrunts_Cue.ZombieGrunts_Cue" (`SceneComponent.K2_GetComponentLocation` (`self.CapsuleComponent`)) (struct) 1.0 1.0 0.0 null null null null :!label _label_2)
  (`KismetSystemLibrary.Delay` (`KismetMathLibrary.Conv_IntToDouble` (+ (`KismetMathLibrary.RandomInteger` 3) 1)))
  (goto _label_2))

(event `self.ReceiveTick`
  (params (DeltaSeconds :type "Float (single-precision)"))
  (bind _returnvalue (`KismetMathLibrary.MakeVector` 1.0 1.0))
  (bind _returnvalue_2 (`GameplayStatics.GetPlayerPawn` 0))
  (bind _health_bar_widget (`self.Health Bar Widget`))
  (`|ExecutionSequence`
    (:`then_0`
      ; How it decides to shoot vs moving toawrds the player
      (set `self.CanAttack` true)
      (if (> (`KismetMathLibrary.VSize` (- (`SceneComponent.K2_GetComponentLocation` (`Actor.RootComponent` _returnvalue_2)) (`SceneComponent.K2_GetComponentLocation` (`self.CapsuleComponent`)))) 1000.0)
        (`|AIMoveTo` self (0.0 0.0 0.0) _returnvalue_2 70.0)
        (else
          (`MovementComponent.StopMovementImmediately` (`self.CharacterMovement`))
          (`self.AttackPLayerForAnim`))))
    (:`then_1`
      ; Looks at the player
      (`SceneComponent.K2_SetWorldRotation` (`self.CapsuleComponent`) (`KismetMathLibrary.FindLookAtRotation` (* (`SceneComponent.K2_GetComponentLocation` (`self.CapsuleComponent`)) _returnvalue) (* _returnvalue (`self.K2_GetActorLocation` (`GameplayStatics.GetPlayerPawn` 0)))) false false))
    (:`then_2`
      (bind _asenemy_health_bar (cast `/Game/UI/EnemyHealthBar` (`WidgetComponent.GetWidget` (`self.Health Bar Widget`))))
      (`ProgressBar.SetPercent` (`/Game/UI/EnemyHealthBar.HealthBar` _asenemy_health_bar) (/ (`self.Health`) 100.0))
      (`SceneComponent.K2_SetWorldRotation` _health_bar_widget (`KismetMathLibrary.FindLookAtRotation` (`SceneComponent.K2_GetComponentLocation` _health_bar_widget) (`SceneComponent.K2_GetComponentLocation` (`PlayerCameraManager.TransformComponent` (`GameplayStatics.GetPlayerCameraManager` 0)))) false false))))

(event `self.CapsuleComponent.OnComponentBeginOverlap`
  (params (OverlappedComponent :type "PrimitiveComponent Object Reference") (OtherActor :type "Actor Object Reference") (OtherComp :type "PrimitiveComponent Object Reference") (OtherBodyIndex :type Integer) (bFromSweep :type Boolean) (SweepResult :type "HitResult Structure (by ref)"))
  ; How it gets hit and take damage
  (bind _asbp_castable (cast `/Game/Blueprints/BP_Castable` OtherActor))
  (if (`/Game/Blueprints/BP_Castable.IsPlayer` _asbp_castable)
    (bind _output_get (set `self.Health` (- (`self.Health`) 50.0)))
    (if (<= _output_get 0.0)
      (`GameplayStatics.PlaySoundAtLocation` "/Game/AudioFiles/DeathFromSpiritBall.DeathFromSpiritBall" (`SceneComponent.K2_GetComponentLocation` (`self.CapsuleComponent`)) (struct) 1.0 1.0 0.0 null null null null)
      (`self.K2_DestroyActor`))))

(fn `UserConstructionScript`)