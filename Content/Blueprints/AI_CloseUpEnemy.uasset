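; AI_CloseUpEnemy is a melee enemy that chases the player and grunts at random intervals.
; Tick reissues AIMoveTo and resets CanAttack; arrival triggers an attack montage gated by DoOnce, with no damage applied here.
; Player-owned BP_Castable overlaps drain Health until it dies with a sound, while an older Hit event destroys it on player contact.
; Health bar update logic is disconnected and never runs.
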(event `self.ReceiveHit`
  (params (MyComp :type "PrimitiveComponent Object Reference") (Other :type "Actor Object Reference") (OtherComp :type "PrimitiveComponent Object Reference") (bSelfMoved :type Boolean) (HitLocation :type "Vector Structure") (HitNormal :type "Vector Structure") (NormalImpulse :type "Vector Structure") (Hit :type "HitResult Structure (by ref)"))
  ; Old collision checking
  (if (== OtherComp (`GameplayStatics.GetPlayerPawn` 0))
    (`self.K2_DestroyActor`)))

(event `self.ReceiveBeginPlay`
  ; makes the sound effect for random grunts
  (`GameplayStatics.PlaySoundAtLocation` "/Game/AudioFiles/ZombieGrunts_Cue.ZombieGrunts_Cue" (`SceneComponent.K2_GetComponentLocation` (`self.CapsuleComponent`)) (struct) 1.0 1.0 0.0 null null null null :!label _label)
  (`KismetSystemLibrary.Delay` (`KismetMathLibrary.Conv_IntToDouble` (+ (`KismetMathLibrary.RandomInteger` 3) 1)))
  (goto _label))

(event `self.CapsuleComponent.OnComponentBeginOverlap`
  (params (OverlappedComponent :type "PrimitiveComponent Object Reference") (OtherActor :type "Actor Object Reference") (OtherComp :type "PrimitiveComponent Object Reference") (OtherBodyIndex :type Integer) (bFromSweep :type Boolean) (SweepResult :type "HitResult Structure (by ref)"))
  ; How it gets hit and take damage
  (bind _asbp_castable (cast `/Game/Blueprints/BP_Castable` OtherActor))
  (if (`/Game/Blueprints/BP_Castable.IsPlayer` _asbp_castable)
    (bind _output_get (set `self.Health` (- (`self.Health`) 25.0)))
    (if (<= _output_get 0.0)
      (`GameplayStatics.PlaySoundAtLocation` "/Game/AudioFiles/DeathFromSpiritBall.DeathFromSpiritBall" (`SceneComponent.K2_GetComponentLocation` (`self.CapsuleComponent`)) (struct) 1.0 1.0 0.0 null null null null)
      (`self.K2_DestroyActor`))))

(event `self.ReceiveTick`
  (params (DeltaSeconds :type "Float (single-precision)"))
  ; Chases player, then checks if it can attack
  (set `self.canAttack` true)
  (`|AIMoveTo` self (0.0 0.0 0.0) (`GameplayStatics.GetPlayerPawn` 0) 150.0
    (:`OnSuccess`
      (if (`self.canAttack`)
        (set `self.canAttack` false)
        (`self.AttackPlayer`)))))

(event `AttackPlayer`
  ; Preforms attack animation
  (`/Engine/EditorBlueprintResources/StandardMacros.DoOnce` false :!label _label_2
    (:`Completed`
      (bind _returnvalue (`self.PlayAnimMontage` "/Game/animations/Beast_animations/MutantAttackMontage.MutantAttackMontage"))
      (`KismetSystemLibrary.Delay` _returnvalue)
      (set `self.canAttack` true)
      (goto _label_2 :!via `Reset`))))

(fn `UserConstructionScript`)