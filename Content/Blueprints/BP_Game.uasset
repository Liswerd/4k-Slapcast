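; BP_Game manages run state for a game played through a shuffled sequence of room levels, tracking level order, loaded-level count and player health.
; ChangeLevel opens the next entry in Levels, calling Randomize once the list is exhausted.
; Randomize resets the index and health, reshuffling until the first room differs from the current one.
; PlayerHurt decrements health and opens the menu when it runs out.
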(fn `ChangeLevel`
  (bind _levelindex (`self.LevelIndex`))
  (bind _levels (`self.Levels`))
  (if (<= (`KismetArrayLibrary.Array_Length` _levels) _levelindex)
    (`self.Randomize`))
  (bind _output_get (set `self.CurrentLevel` (`|GetArrayItem` _levels _levelindex)))
  (`/Engine/EditorBlueprintResources/StandardMacros.IncrementInt` (`self.LevelIndex`)
    (:`  `
      (`GameplayStatics.OpenLevelBySoftObjectPtr` _output_get))))

(fn `LevelLoaded`
  (`/Engine/EditorBlueprintResources/StandardMacros.IncrementInt` (`self.LevelNum`)))

(fn `PlayerHurt`
  (bind _result (`/Engine/EditorBlueprintResources/StandardMacros.DecrementInt` (`self.PlayerHealth`))
    (:`  `
      (if (<= _result 0)
        (`GameplayStatics.OpenLevelBySoftObjectPtr` (`self.Menu`))))))

(fn `Randomize`
  (bind _levels (`self.Levels`))
  (set `self.LevelIndex` 0)
  (set `self.PlayerHealth` 3)
  (`KismetArrayLibrary.Array_Shuffle` _levels :!label _label)
  (if (== (`|GetArrayItem` _levels) (`self.CurrentLevel`))
    (`KismetSystemLibrary.PrintString` "Rerolled rooms")
    (goto _label)))