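; Enemy actor Blueprint that turns to face the player and destroys itself when its capsule is hit.
; Tick rotates the root toward the player pawn with Z zeroed on both positions, keeping the look-at horizontal.
; Run-and-shoot logic is unfinished: its delayed call is disconnected, RunAtPlayer would snap straight to the player's location, and Shoot's projectile spawn is unwired.
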(event `self.ReceiveTick`
  (params (DeltaSeconds :type "Float (single-precision)"))
  (bind _returnvalue (`KismetMathLibrary.MakeVector` 1.0 1.0))
  (`SceneComponent.K2_SetWorldRotation` (`self.DefaultSceneRoot`) (`KismetMathLibrary.FindLookAtRotation` (* (`SceneComponent.K2_GetComponentLocation` (`self.DefaultSceneRoot`)) _returnvalue) (* _returnvalue (`self.K2_GetActorLocation` (`GameplayStatics.GetPlayerPawn` 0)))) false false))

(event `self.Capsule.OnComponentHit`
  (params (HitComponent :type "PrimitiveComponent Object Reference") (OtherActor :type "Actor Object Reference") (OtherComp :type "PrimitiveComponent Object Reference") (NormalImpulse :type "Vector Structure") (Hit :type "HitResult Structure (by ref)"))
  (`self.K2_DestroyActor`))

(fn `RunAndShootAtPlayer`
  (`self.RunAtPlayer`)
  (`self.Shoot`))

(fn `RunAtPlayer`
  (`self.K2_SetActorLocation` (`self.K2_GetActorLocation` (`GameplayStatics.GetPlayerPawn` 0))))

(fn `Shoot`)

(fn `UserConstructionScript`)