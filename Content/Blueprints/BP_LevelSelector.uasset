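; BP_LevelSelector moves the game to a randomly picked level once all enemies in the current one are gone.
; While its SpawnedEnemies flag is set, Tick polls GetAllActorsOfClass for three enemy classes: BP_Enemy, AI_CloseUpEnemy and AI_ShootingEnemy.
; When none remain, it opens a random entry from Levels and plays the Chakraopen sound.
; The flag is not set within this Blueprint.
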(event `self.ReceiveBeginPlay`
  (`parent.ReceiveBeginPlay`))

(event `self.ReceiveTick`
  (params (DeltaSeconds :type "Float (single-precision)"))
  (`parent.ReceiveTick` DeltaSeconds)
  (if (`self.SpawnedEnemies`)
    (bind _outactors (`GameplayStatics.GetAllActorsOfClass` "/Game/Blueprints/BP_Enemy.BP_Enemy_C"))
    (bind _outactors_2 (`GameplayStatics.GetAllActorsOfClass` "/Game/Blueprints/AI_CloseUpEnemy.AI_CloseUpEnemy_C"))
    (bind _outactors_3 (`GameplayStatics.GetAllActorsOfClass` "/Game/Blueprints/AI_ShootingEnemy.AI_ShootingEnemy_C"))
    (if (and (== (`KismetArrayLibrary.Array_Length` _outactors) 0) (== (`KismetArrayLibrary.Array_Length` _outactors_2) 0) (== (`KismetArrayLibrary.Array_Length` _outactors_3) 0))
      (`GameplayStatics.OpenLevelBySoftObjectPtr` (`KismetArrayLibrary.Array_Random` (`self.Levels`)))
      (`GameplayStatics.PlaySound2D` "/Game/AudioFiles/chakraopen.chakraopen" 1.0 1.0 0.0 null null))))

(fn `UserConstructionScript`
  (`parent.UserConstructionScript`))