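; SpiritBall is a skill Blueprint that fires a spirit ball projectile on behalf of the player.
; On ExecCast it plays a grunt sound at the start point and spawns a BP_SpiritBallObject slightly ahead along the direction to the end point.
; It marks the spawned object as player-made and sets its velocity along that direction, scaled by Speed.
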(event `self.ExecCast`
  (params (start :type "Vector Structure") (end :type "Vector Structure"))
  (bind _returnvalue (`KismetMathLibrary.Normal` (- end start)))
  (`GameplayStatics.PlaySoundAtLocation` "/Game/AudioFiles/PlayerGrunt_Cue.PlayerGrunt_Cue" start (struct) 1.0 1.0 0.0 null null null null)
  (bind _returnvalue_2 (`|SpawnActorFromClass` "/Game/Blueprints/BP_SpiritBallObject.BP_SpiritBallObject_C" (`KismetMathLibrary.MakeTransform` (+ start (* _returnvalue (`KismetMathLibrary.Conv_DoubleToVector` 100.0)))) "AdjustIfPossibleButAlwaysSpawn" "MultiplyWithRoot" null null))
  (`/Game/Blueprints/BP_Castable.MakeFromPlayer` _returnvalue_2)
  (`/Game/Blueprints/BP_SpiritBallObject.SetVelocity` _returnvalue_2 (* _returnvalue (`self.Speed`))))

(fn `UserConstructionScript`)