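; Wall skill Blueprint that summons a wall in front of the player when cast.
; ExecCast plays a grunt sound at the given start location, then spawns BP_WallSummon 100 units from it along the player's forward direction, matching the pawn's rotation.
; The summon attaches to the player pawn with world transform kept, so it moves with the player from its spawn offset.
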(event `self.ExecCast`
  (params (start :type "Vector Structure") (end :type "Vector Structure"))
  (bind _returnvalue (`Actor.K2_GetActorRotation` (`GameplayStatics.GetPlayerPawn` 0)))
  (`GameplayStatics.PlaySoundAtLocation` "/Game/AudioFiles/PlayerGrunt_Cue.PlayerGrunt_Cue" start (struct) 1.0 1.0 0.0 null null null null)
  (bind _returnvalue_2 (`|SpawnActorFromClass` "/Game/Blueprints/BP_WallSummon.BP_WallSummon_C" (`KismetMathLibrary.MakeTransform` (+ start (* (`KismetMathLibrary.Normal` (`KismetMathLibrary.GetForwardVector` _returnvalue)) (`KismetMathLibrary.Conv_DoubleToVector` 100.0))) _returnvalue) "AdjustIfPossibleButAlwaysSpawn" "MultiplyWithRoot" null null))
  (`Actor.K2_AttachToActor` _returnvalue_2 (`GameplayStatics.GetPlayerPawn` 0) "None" "KeepWorld" "KeepWorld" "KeepWorld" true))

(fn `UserConstructionScript`)