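; BP_ConeBlast is a short-lived cone blast actor with a cast sound at the player pawn's location.
; BeginPlay waits briefly, plays CastCone, then destroys the actor about a second later.
; SetVelocity lets a caller drive the MoveConeASmidge component.
; The Box overlap handler has no effect; the cursor-aimed velocity logic and AI_ShootingEnemy cast are disconnected.
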(event `self.ReceiveBeginPlay`
  (`KismetSystemLibrary.Delay` 0.05)
  (`GameplayStatics.PlaySoundAtLocation` "/Game/AudioFiles/CastCone.CastCone" (`self.K2_GetActorLocation` (`GameplayStatics.GetPlayerPawn` 0)) (struct) 1.0 1.0 0.0 null null null null)
  (`KismetSystemLibrary.Delay` 1.0)
  (`self.K2_DestroyActor`))

(event `self.Box.OnComponentBeginOverlap`
  (params (OverlappedComponent :type "PrimitiveComponent Object Reference") (OtherActor :type "Actor Object Reference") (OtherComp :type "PrimitiveComponent Object Reference") (OtherBodyIndex :type Integer) (bFromSweep :type Boolean) (SweepResult :type "HitResult Structure (by ref)"))
  (if true
    _))

(fn `SetVelocity`
  (params (Velocity :type "Vector Structure"))
  (set `MovementComponent.Velocity` Velocity (`self.MoveConeASmidge`)))

(fn `UserConstructionScript`)