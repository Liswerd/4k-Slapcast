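; Enemy spawner actor that repeatedly spawns batches of a configurable actor class at random positions.
; Tick runs a Delay into Spawn, so a batch appears roughly every WaitToSpawnDuration.
; Randomize offsets X and Y by up to Range in one direction from the spawner's location or a set Origin, keeping that Z.
; Spawn moves each actor to that point, then increments and prints NumSpawned once per batch.
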(event `self.ReceiveBeginPlay`)

(event `self.ReceiveTick`
  (params (DeltaSeconds :type "Float (single-precision)"))
  (`KismetSystemLibrary.Delay` (`self.waitToSpawnDuration`))
  (`self.Spawn`))

(fn `Randomize`
  (returns (RandomizedPosition :type "Vector Structure"))
  (if (`self.useThisAsOrigin`)
    (return (`KismetMathLibrary.MakeVector` (+ (* (.x (`self.range`)) (`KismetMathLibrary.RandomFloat`)) (.x (`self.K2_GetActorLocation`))) (+ (* (.y (`self.range`)) (`KismetMathLibrary.RandomFloat`)) (.y (`self.K2_GetActorLocation`))) (.z (`self.K2_GetActorLocation`))))
    (else
      (return (`KismetMathLibrary.MakeVector` (+ (* (.x (`self.range`)) (`KismetMathLibrary.RandomFloat`)) (.x (`self.origin`))) (+ (* (.y (`self.range`)) (`KismetMathLibrary.RandomFloat`)) (.y (`self.origin`))) (.z (`self.origin`)))))))

(fn `Spawn`
  (bind _tospawn (`self.ToSpawn`))
  (for _ (range (`self.numToSpawn`))
    (bind _randomizedposition (`self.Randomize`))
    (if (`self.useThisAsOrigin`)
      (bind _returnvalue (`|SpawnActorFromClass` _tospawn (`KismetMathLibrary.Conv_VectorToTransform` (`self.K2_GetActorLocation`)) "Undefined" "MultiplyWithRoot" null null))
      (`self.K2_SetActorLocation` _returnvalue _randomizedposition false false)
      (else
        (bind _returnvalue_2 (`|SpawnActorFromClass` _tospawn (`KismetMathLibrary.Conv_VectorToTransform` _randomizedposition) "Undefined" "MultiplyWithRoot" null null))
        (`self.K2_SetActorLocation` _returnvalue_2 _randomizedposition false false))))
  (bind _output_get (set `self.numSpawned` (+ (`self.numSpawned`) 1)))
  (`KismetSystemLibrary.PrintString` (`KismetStringLibrary.BuildString_Int` "" "SPAWNED #" _output_get)))

(fn `UserConstructionScript`)