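; BP_SpiritBallObject is a spirit ball projectile that plays a throw sound at the player pawn's location shortly after spawning.
; SetVelocity assigns the supplied vector directly to its ProjectileMovement, so the caller controls direction and speed.
; Its Box overlap destroys the ball one tick after touching anything except another spirit ball.
; Older cursor-aiming, impact-effect and debug logic remains disconnected in the event graph.
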(event `self.ReceiveBeginPlay`
  (`KismetSystemLibrary.Delay` 0.05)
  (`GameplayStatics.PlaySoundAtLocation` "/Game/AudioFiles/ProjectileThrow_Cue.ProjectileThrow_Cue" (`self.K2_GetActorLocation` (`GameplayStatics.GetPlayerPawn` 0)) (struct) 1.0 1.0 0.0 null null null null))

(event `self.Box.OnComponentBeginOverlap`
  (params (OverlappedComponent :type "PrimitiveComponent Object Reference") (OtherActor :type "Actor Object Reference") (OtherComp :type "PrimitiveComponent Object Reference") (OtherBodyIndex :type Integer) (bFromSweep :type Boolean) (SweepResult :type "HitResult Structure (by ref)"))
  (if (not (`GameplayStatics.ObjectIsA` OtherActor "BP_SpiritBallObject_C"))
    (`KismetSystemLibrary.DelayUntilNextTick`)
    (`self.K2_DestroyActor`)))

(event `self.ReceiveActorBeginOverlap`
  (params (OtherActor :type "Actor Object Reference")))

(fn `SetVelocity`
  (params (Direction :type "Vector Structure"))
  (set `MovementComponent.Velocity` Direction (`self.ProjectileMovement`)))

(fn `UserConstructionScript`)