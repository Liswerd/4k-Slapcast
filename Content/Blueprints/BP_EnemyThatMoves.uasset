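; Enemy Blueprint intended to chase the player, though its movement node is not connected.
; On BeginPlay, MoveToPlayer casts player pawn 0 to PlayerPawn and caches the reference.
; Every Tick, GetPlayerPosition stores that pawn's location in PlayerPOSITION.
; An AI MoveTo node takes both values as target and destination but never executes, so this graph only tracks the player.
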(event `move to player`
  (bind _asplayer_pawn (cast `PlayerPawn` (`GameplayStatics.GetPlayerPawn` 0)))
  (bind _output_get (set `self.As Player Pawn` _asplayer_pawn)))

(event `self.ReceiveBeginPlay`
  (`self.move to player`))

(event `get player position`
  (set `self.Player POSITION` (`self.K2_GetActorLocation` (`self.As Player Pawn`))))

(event `self.ReceiveTick`
  (params (DeltaSeconds :type "Float (single-precision)"))
  (`self.get player position`))

(fn `UserConstructionScript`)