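; BP_WallSummon is a temporary summoned wall actor that plays a cast sound at the player's location shortly after spawning.
; After about four seconds it spawns a Niagara collapse effect at its own location and destroys itself.
; When a spirit ball object begins overlapping its Box component, it plays a 2D blocked sound; the graph applies no other effect to the ball.
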(event `self.ReceiveBeginPlay`
  (`KismetSystemLibrary.Delay` 0.05)
  (`GameplayStatics.PlaySoundAtLocation` "/Game/AudioFiles/CastWall.CastWall" (`self.K2_GetActorLocation` (`GameplayStatics.GetPlayerPawn` 0)) (struct) 1.0 1.0 0.0 null null null null)
  (`KismetSystemLibrary.Delay` 4.0)
  (`NiagaraFunctionLibrary.SpawnSystemAtLocation` "/Game/ParticleEffect/NS_collapse.NS_collapse" (`self.K2_GetActorLocation`))
  (`self.K2_DestroyActor`))

(event `self.Box.OnComponentBeginOverlap`
  (params (OverlappedComponent :type "PrimitiveComponent Object Reference") (OtherActor :type "Actor Object Reference") (OtherComp :type "PrimitiveComponent Object Reference") (OtherBodyIndex :type Integer) (bFromSweep :type Boolean) (SweepResult :type "HitResult Structure (by ref)"))
  (if (`GameplayStatics.ObjectIsA` OtherActor "/Game/Blueprints/BP_SpiritBallObject.BP_SpiritBallObject_C")
    (`GameplayStatics.PlaySound2D` "/Game/AudioFiles/WallBlocked_Cue.WallBlocked_Cue" 1.0 1.0 0.0 null null)))

(fn `UserConstructionScript`)